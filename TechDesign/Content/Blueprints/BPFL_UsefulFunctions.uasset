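; Blueprint function library of shared helpers for a tile-based building game with build, road and demo modes.
; Mode queries and toggles forward to the game mode through message calls, so callers need no direct reference to it.
; Other helpers show or hide the cursor, add or remove the build-mode input mapping context, and return the actor under the cursor if tagged as a Tile.
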(fn ToggleMouse
  (params (Show? :type Boolean))
  (Variables|/Script/Engine.PlayerController|SetbShowMouseCursor (Game|GetPlayerController 0) Show?)
  (return))

(fn ToggleBuildModeControls
  (params (Enable? :type Boolean))
  (if Enable?
    (Input|AddMappingContext (PlayerController|LocalPlayerSubsystems|GetEnhancedInputLocalPlayerSubsystem (Game|GetPlayerController 0)) "/Game/Blueprints/Input/BuildMode/IMC_BuildMode.IMC_BuildMode" 0 "(bIgnoreAllPressedKeysUntilRelease=True,bForceImmediately=False,bNotifyUserSettings=False)")
    (else
      (Input|RemoveMappingContext (PlayerController|LocalPlayerSubsystems|GetEnhancedInputLocalPlayerSubsystem (Game|GetPlayerController 0)) "/Game/Blueprints/Input/BuildMode/IMC_BuildMode.IMC_BuildMode" "(bIgnoreAllPressedKeysUntilRelease=True,bForceImmediately=False,bNotifyUserSettings=False)"))))

(fn PlayerinBuildMode?
  (bind _in_build_mode_ (Class|BPIQuery|InBuildMode?(Message) (Game|GetGameMode)))
  (return _in_build_mode_))

(fn PlayerinRoadMode?
  (bind _in_road_mode_ (Class|BPIQuery|InRoadMode?(Message) (Game|GetGameMode)))
  (return _in_road_mode_))

(fn PlayerinDemoMode?
  (bind _in_demo_mode_ (Class|BPIQuery|InDemoMode?(Message) (Game|GetGameMode)))
  (return _in_demo_mode_))

(fn ToggleBuildMode
  (params (On? :type Boolean))
  (Class|BPIBuild|ToggleBuildMode(Message) (Game|GetGameMode) On?))

(fn ToggleRoadMode
  (params (On? :type Boolean))
  (Class|BPIBuild|ToggleRoadMode(Message) (Game|GetGameMode) On?))

(fn ToggleDemoMode
  (params (On? :type Boolean))
  (Class|BPIBuild|ToggleDemoMode(Message) (Game|GetGameMode) On?))

(fn GetTileUnderMouse
  (bind _returnvalue (Game|GetPlayerController 0))
  (bind _hitresult (Game|Player|GetHitResultUnderCursorbyChannel _returnvalue "TraceTypeQuery1" true))
  (bind _hitactor (Collision|BreakHitResult _hitresult))
  (if (Actor|ActorHasTag _hitactor "Tile")
    (return _hitactor)))