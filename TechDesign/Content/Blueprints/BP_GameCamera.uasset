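; Player camera pawn for a tile-based building game, handling view control and building placement input.
; Enhanced Input drives yaw-relative movement, spring-arm zoom and hold-to-pan orbit with clamped pitch.
; Clicks trace under the cursor, then check build mode, affordability, tile occupancy and the building's road, neighbour or limit rules.
; Placement and rotation requests go to the GameMode as messages, with sounds for click feedback.
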(event Input|EnhancedActionEvents|EnhancedInputActionIA_Move
  (params (ActionValue :type Vector%202D%20Structure) (ElapsedSeconds :type Float%20%28double-precision%29) (TriggeredSeconds :type Float%20%28double-precision%29) (InputAction :type Input%20Action%20Object%20Reference :default "/Game/Blueprints/Input/IA_Move.IA_Move"))
  (bind _springarm (Variables|Default|GetSpringArm))
  (bind _relativerotation (Variables|/Script/Engine.SceneComponent|GetRelativeRotation _springarm))
  (Class|PawnMovementComponent|AddInputVector (Variables|Default|GetFloatingPawnMovement) (Math|Vector|RotateVector (Math|Conversions|ToVector(Vector2D) ActionValue) (Math|Rotator|MakeRotator (.roll _relativerotation) (.pitch (Transformation|GetActorRotation)) (.yaw _relativerotation))) false))

(event Input|EnhancedActionEvents|EnhancedInputActionIA_Click
  (params (ActionValue :type Boolean) (ElapsedSeconds :type Float%20%28double-precision%29) (TriggeredSeconds :type Float%20%28double-precision%29) (InputAction :type Input%20Action%20Object%20Reference :default "/Game/Blueprints/Input/IA_Click.IA_Click"))
  (bind _returnvalue (Game|GetPlayerController 0))
  (bind _hitresult (Game|Player|GetHitResultUnderCursorbyChannel _returnvalue "TraceTypeQuery1" true))
  (bind _hitactor (Collision|BreakHitResult _hitresult))
  (:Started
    (bind _place_ (CallFunction|CanBuildingbePlaced? _hitactor))
    (if _place_
      (Class|BPIBuild|PlaceBuilding(Message) (Game|GetGameMode) _hitactor)
      (Audio|PlaySound2D "/Game/Assets/Sound/SFX/JDSherbert_WoodenSFX/A_Confirm3.A_Confirm3" 1.0 1.0 0.0 0 0)
      (elif (not (or (CallFunction|PlayerinRoadMode?) (CallFunction|PlayerinDemoMode?)))
        (Audio|PlaySound2D "/Game/Assets/Sound/SFX/JDSherbert_WoodenSFX/A_Cursor3.A_Cursor3" 1.0 1.0 0.0 0 0)))))

(event Input|EnhancedActionEvents|EnhancedInputActionIA_Zoom
  (params (ActionValue :type Float%20%28double-precision%29) (ElapsedSeconds :type Float%20%28double-precision%29) (TriggeredSeconds :type Float%20%28double-precision%29) (InputAction :type Input%20Action%20Object%20Reference :default "/Game/Blueprints/Input/IA_Zoom.IA_Zoom"))
  (:Started
    (Variables|/Script/Engine.SpringArmComponent|SetTargetArmLength (Variables|Default|GetSpringArm) (Math|Float|Clamp(Float) (+ (Variables|/Script/Engine.SpringArmComponent|GetTargetArmLength (Variables|Default|GetSpringArm)) (* ActionValue -2.5e+02)) 0.0 2e+03))))

(event Input|EnhancedActionEvents|EnhancedInputActionIA_Pan
  (params (ActionValue :type Vector%202D%20Structure) (ElapsedSeconds :type Float%20%28double-precision%29) (TriggeredSeconds :type Float%20%28double-precision%29) (InputAction :type Input%20Action%20Object%20Reference :default "/Game/Blueprints/Input/IA_Pan.IA_Pan"))
  (bind _returnvalue (* ActionValue 2.0))
  (bind _springarm (Variables|Default|GetSpringArm))
  (bind (_x _y) (Math|Vector2D|BreakVector2D _returnvalue))
  (bind _returnvalue_2 (Transformation|GetWorldRotation _springarm))
  (if (Variables|Default|GetCan%20Pan?)
    (Transformation|SetWorldRotation _springarm (Math|Rotator|MakeRotator (.roll _returnvalue_2) (Math|Float|Clamp(Float) (+ (.pitch _returnvalue_2) _y) -6e+01 -2e+01) (+ (.yaw _returnvalue_2) _x)) false false)))

(event Input|EnhancedActionEvents|EnhancedInputActionIA_PanToggle
  (params (ActionValue :type Boolean) (ElapsedSeconds :type Float%20%28double-precision%29) (TriggeredSeconds :type Float%20%28double-precision%29) (InputAction :type Input%20Action%20Object%20Reference :default "/Game/Blueprints/Input/IA_PanToggle.IA_PanToggle"))
  (:Started
    (CallFunction|ToggleMouse false)
    (Variables|Default|SetCan%20Pan? true))
  (:Completed
    (CallFunction|ToggleMouse true)
    (Variables|Default|SetCan%20Pan? false)))

(event Input|EnhancedActionEvents|EnhancedInputActionIA_RotateCW
  (params (ActionValue :type Boolean) (ElapsedSeconds :type Float%20%28double-precision%29) (TriggeredSeconds :type Float%20%28double-precision%29) (InputAction :type Input%20Action%20Object%20Reference :default "/Game/Blueprints/Input/BuildMode/IA_RotateCW.IA_RotateCW"))
  (:Started
    (if (CallFunction|PlayerinBuildMode?)
      (Class|BPIBuild|RotateBuilding(Message) (Game|GetGameMode) false))))

(event Input|EnhancedActionEvents|EnhancedInputActionIA_RotateCCW
  (params (ActionValue :type Boolean) (ElapsedSeconds :type Float%20%28double-precision%29) (TriggeredSeconds :type Float%20%28double-precision%29) (InputAction :type Input%20Action%20Object%20Reference :default "/Game/Blueprints/Input/BuildMode/IA_RotateCCW.IA_RotateCCW"))
  (:Started
    (if (CallFunction|PlayerinBuildMode?)
      (Class|BPIBuild|RotateBuilding(Message) (Game|GetGameMode) true))))

(event EventBeginPlay
  (CallFunction|ToggleMouse true)
  (Input|AddMappingContext (PlayerController|LocalPlayerSubsystems|GetEnhancedInputLocalPlayerSubsystem (Game|GetPlayerController 0)) "/Game/Blueprints/Input/IMC_Default.IMC_Default" 0 "(bIgnoreAllPressedKeysUntilRelease=True,bForceImmediately=False,bNotifyUserSettings=False)"))

(fn ConstructionScript)

(fn CanBuildingbePlaced?
  (params (Tile :type Actor%20Object%20Reference))
  (bind _returnvalue (Game|GetGameMode))
  (bind _rules_followed_ (CallFunction|PlacementRulesFulfiled? Tile))
  (bind _is_occupied_ (Class|BPIQuery|TileOccupied?(Message) Tile))
  (bind _in_build_mode_ (Class|BPIQuery|InBuildMode?(Message) _returnvalue))
  (bind _can_afford_ (Class|BPIQuery|CanPlayerAfford?(Message) _returnvalue))
  (return (Math|Boolean|ANDBoolean _can_afford_ _in_build_mode_ (not _is_occupied_) _rules_followed_)))

(fn PlacementRulesFulfiled?
  (params (Tile :type Actor%20Object%20Reference))
  (LocalVariables|SetL%20Tile Tile)
  (LocalVariables|SetL%20Rules true)
  (bind _current_building (Class|BPIGetters|GetCurrentBuildingtoPlace(Message) (Game|GetGameMode)))
  (bind _output_get (LocalVariables|SetL%20Current%20Building _current_building))
  (bind (_rules _rule_bps) (Class|BPIGetters|GetPlacementRules(Message) _output_get))
  (LocalVariables|SetL%20Rule%20BPs _rule_bps)
  (for _array_element _rules
    (switch Utilities|FlowControl|Switch|SwitchonE_PlacementRule _array_element
      (:NewEnumerator0
        (bind _road_adjacent_ (Class|BPIQuery|AdjacenttoRoad?(Message) (LocalVariables|GetL%20Tile)))
        (if (not _road_adjacent_)
          (LocalVariables|SetL%20Rules false :!label _label)))
      (:NewEnumerator2
        (bind _bp_adjacent_ (Class|BPIQuery|IsAdjacenttoRuleBP?(Message) (LocalVariables|GetL%20Tile) (LocalVariables|GetL%20Rule%20BPs)))
        (if (not _bp_adjacent_)
          (goto _label)))
      (:NewEnumerator1
        (bind _placed_buildings (Class|BPIGetters|GetPlacedBuildingsArray(Message) (Game|GetGameMode)))
        (for _array_element_2 _placed_buildings
          (if (== (Utilities|GetClass _array_element_2) (Utilities|GetClass (LocalVariables|GetL%20Current%20Building)))
            (goto _label))))))
  (return (LocalVariables|GetL%20Rules)))