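; Hex grid tile for a building game that shows a mode-coloured hover overlay and handles road placement, road removal and building demolition on click.
; It tracks type, occupant and six neighbours, notifying neighbours when roads change and answering adjacency queries.
; Road auto-tiling builds a six-bit neighbour mask, cycles it to match a default pattern, then sets the mesh and yaw in 60-degree steps.
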(event OnBeginCursorOver(Hex)
  (params (TouchedComponent :type Primitive%20Component%20Object%20Reference))
  (CallFunction|HoverOverlay true))

(event OnEndCursorOver(Hex)
  (params (TouchedComponent :type Primitive%20Component%20Object%20Reference))
  (CallFunction|HoverOverlay false)
  (Utilities|IsValid (Variables|Default|GetPrevious%20Building)
    (:Is%20Valid
      (Class|BPIBuild|DemolitionPreview(Message) (Variables|Default|GetPrevious%20Building) false)
      (Class|BPIBuild|ToggleBuildingCollisions(Message) (Variables|Default|GetPrevious%20Building) true)
      (Variables|Default|SetPrevious%20Building 0))))

(event OnClicked(Hex)
  (params (TouchedComponent :type Primitive%20Component%20Object%20Reference) (ButtonPressed :type Key%20Structure))
  (bind _tile_data (Variables|Default|GetTile%20Data))
  (bind _occupyingactor (Utilities|Struct|BreakS_TileData _tile_data))
  (if (CallFunction|PlayerinRoadMode?)
    (CallFunction|PlaceRoad)
    (CallFunction|UpdateRoad)
    (Default|CallEvent:NeighbourRoadUpdated)
    (elif (CallFunction|PlayerinDemoMode?)
      (switch Utilities|FlowControl|Switch|SwitchonE_TileType (Utilities|Struct|BreakS_TileData (Variables|Default|GetTile%20Data))
        (:NewEnumerator0
          (Utilities|IsValid _occupyingactor
            (:Is%20Valid
              (Class|BPIBuild|RemoveBuilding(Message) _occupyingactor)
              (Utilities|Struct|SetmembersinS_TileData (Variables|Default|GetTile%20Data) false))))
        (:NewEnumerator1
          (CallFunction|RemoveRoad)
          (Default|CallEvent:NeighbourRoadUpdated))))))

(event Custom|Init:%20Event%20Bindings
  (bind _tile_neighbour (Variables|Default|GetTile%20Neighbour))
  (bind (_nneighbour _neneighbour _seneighbour _sneighbour _swneighbour _nwneighbour) (Utilities|Struct|BreakS_TileNeighbour _tile_neighbour))
  (for _array_element (Utilities|Array|MakeArray _nneighbour _neneighbour _seneighbour _sneighbour _swneighbour _nwneighbour)
    (Utilities|IsValid _array_element
      (:Is%20Valid
        (EventDispatchers|BindEventtoEvent:NeighbourRoadUpdated _array_element (EventDispatchers|CreateEvent :!event UpdateRoad))))))

(event EventBeginPlay
  (Variables|Default|SetOutline (Variables|Default|GetWidget)))

(event EventToggleTileOverlay
  (params (Visible? :type Boolean))
  (CallFunction|HoverOverlay Visible?))

(event EventUpdateTileData
  (params (New%20Occupation :type Boolean) (Building%20Ref :type Actor%20Object%20Reference))
  (Utilities|Struct|SetmembersinS_TileData (Variables|Default|GetTile%20Data) New%20Occupation Building%20Ref))

(fn ConstructionScript)

(fn HoverOverlay
  (params (Visible? :type Boolean))
  (CallFunction|UpdateOverlayColour)
  (Rendering|SetVisibility (Variables|Default|GetWidget) Visible? false))

(fn ReturntoGrassTile
  (if (not (Utilities|Enum|Equal(Enum) (Utilities|Struct|BreakS_TileData (Variables|Default|GetTile%20Data)) "NewEnumerator1"))
    (Rendering|SetVisibility (Variables|Default|GetWidget) false false)))

(fn PlaceRoad
  (bind _tile_data (Variables|Default|GetTile%20Data))
  (bind (_tiletype _occupied_) (Utilities|Struct|BreakS_TileData _tile_data))
  (if (not (and (Utilities|Enum|Equal(Enum) _tiletype "NewEnumerator0") _occupied_))
    (Components|StaticMesh|SetStaticMesh (Variables|Default|GetHex) "/Game/Assets/Tiles/Roads/SM_hex_road_A.SM_hex_road_A")
    (Utilities|Struct|SetmembersinS_TileData (Variables|Default|GetTile%20Data) "NewEnumerator1" true)
    (CallFunction|UpdateOverlayColour)))

(fn GetRoadMask
  (params (Rotation%20Order :type Array%20of%20Integers))
  (bind _tile_neighbour (Variables|Default|GetTile%20Neighbour))
  (bind (_nneighbour _neneighbour _seneighbour _sneighbour _swneighbour _nwneighbour) (Utilities|Struct|BreakS_TileNeighbour _tile_neighbour))
  (LocalVariables|SetL%20Road%20Mask 0)
  (for (_array_element _array_index) Rotation%20Order
    (Utilities|IsValid (Utilities|Array|Get(acopy) (Utilities|Array|MakeArray _nneighbour _neneighbour _seneighbour _sneighbour _swneighbour _nwneighbour) _array_element)
      (:Is%20Valid
        (if (Utilities|Enum|Equal(Enum) (.TileType (Utilities|Struct|BreakS_TileData (Variables|BP_HexTile_C|GetTile%20Data (Utilities|Array|Get(acopy) (Utilities|Array|MakeArray _nneighbour _neneighbour _seneighbour _sneighbour _swneighbour _nwneighbour) _array_element)))) "NewEnumerator1")
          (LocalVariables|SetL%20Road%20Mask (Class|KismetMathLibrary|OrIntInt (|BitmaskLiteral (LocalVariables|GetL%20Road%20Mask)) (Math|Float|Truncate (Math|Float|Power 2.0 (Math|Conversions|ToFloat(Integer) _array_index)))))))))
  (return (LocalVariables|GetL%20Road%20Mask)))

(fn FindRoadMesh
  (params (Road%20Mask :type Integer))
  (return (.Value (Utilities|Map|Find (LocalVariables|GetL%20Mask%20and%20Mesh) Road%20Mask))))

(fn UpdateRoad
  (if (Utilities|Enum|Equal(Enum) (Utilities|Struct|BreakS_TileData (Variables|Default|GetTile%20Data)) "NewEnumerator1")
    (bind _road_mask (CallFunction|GetRoadMask (Utilities|Array|MakeArray 0 1 2 3 4 5)))
    (bind _output_get (LocalVariables|SetRoad%20Mask _road_mask))
    (bind (_road_mask_2 _rotation) (CallFunction|FindCorrectRotation _output_get))
    (Transformation|SetActorRotation (Math|Rotator|MakeRotator 0.0 0.0 _rotation))
    (bind _road_mesh (CallFunction|FindRoadMesh _road_mask_2))
    (Components|StaticMesh|SetStaticMesh (Variables|Default|GetHex) _road_mesh)))

(fn FindCorrectRotation
  (params (Initial%20Road%20Mask :type Integer))
  (LocalVariables|SetL%20Rotation%20Steps 0)
  (LocalVariables|SetL%20Rotation%20Order (Utilities|Array|MakeArray 5 0 1 2 3 4))
  (bind _output_get (LocalVariables|SetL%20Current%20Mask Initial%20Road%20Mask))
  (if (CallFunction|MaskFoundinDefault? _output_get)
    (return (LocalVariables|GetL%20Current%20Mask) 0.0)
    (else
      (Utilities|FlowControl|ForLoopwithBreak 0 5 :!label _label
        (:LoopBody
          (Math|Integer|IncrementInt (LocalVariables|GetL%20Rotation%20Steps)
            (:%20%20
              (bind _road_mask (CallFunction|GetRoadMask (LocalVariables|GetL%20Rotation%20Order)))
              (bind _output_get_2 (LocalVariables|SetL%20Current%20Mask _road_mask))
              (if (CallFunction|MaskFoundinDefault? _output_get_2)
                (goto _label Break)
                (else
                  (bind _new_rotation (CallFunction|CycleRotation (LocalVariables|GetL%20Rotation%20Order)))
                  (LocalVariables|SetL%20Rotation%20Order _new_rotation))))))
        (:Completed
          (return (LocalVariables|GetL%20Current%20Mask) (Math|Conversions|ToFloat(Integer) (* (LocalVariables|GetL%20Rotation%20Steps) -60))))))))

(fn CycleRotation
  (params (Old%20Rotation :type Array%20of%20Integers))
  (bind _output_get (LocalVariables|SetL%20New%20Rotation Old%20Rotation))
  (LocalVariables|SetL%20New%20First%20Index (Utilities|Array|Get(acopy) _output_get 5))
  (Utilities|Array|RemoveIndex (LocalVariables|GetL%20New%20Rotation) 5)
  (Utilities|Array|Insert (LocalVariables|GetL%20New%20Rotation) (LocalVariables|GetL%20New%20First%20Index))
  (return (LocalVariables|GetL%20New%20Rotation)))

(fn MaskFoundinDefault?
  (params (Road%20Mask :type Integer%20%28by%20ref%29))
  (return (Utilities|Array|ContainsItem (LocalVariables|GetL%20Default%20Tile%20Values) Road%20Mask)))

(fn UpdateOverlayColour
  (bind _tile_data (Variables|Default|GetTile%20Data))
  (bind _tile_data_2 (Variables|Default|GetTile%20Data))
  (bind (_tiletype _occupied_) (Utilities|Struct|BreakS_TileData _tile_data_2))
  (bind _occupyingactor (Utilities|Struct|BreakS_TileData _tile_data))
  (if (CallFunction|PlayerinRoadMode?)
    (if (and (Utilities|Enum|Equal(Enum) _tiletype "NewEnumerator0") (not _occupied_))
      (Class|WidgetComponent|SetTintColorandOpacity (Variables|Default|GetWidget) "(R=0.000000,G=1.000000,B=0.000000,A=1.000000)")
      (else
        (Class|WidgetComponent|SetTintColorandOpacity (Variables|Default|GetWidget) "(R=1.000000,G=0.000000,B=0.000000,A=1.000000)")))
    (elif (CallFunction|PlayerinDemoMode?)
      (Class|WidgetComponent|SetTintColorandOpacity (Variables|Default|GetWidget) "(R=1.000000,G=0.995244,B=0.000000,A=1.000000)")
      (Utilities|IsValid _occupyingactor
        (:Is%20Valid
          (bind _output_get (Variables|Default|SetPrevious%20Building _occupyingactor))
          (Class|BPIBuild|DemolitionPreview(Message) _output_get true)
          (Class|BPIBuild|ToggleBuildingCollisions(Message) _output_get false)))
      (else
        (Class|WidgetComponent|SetTintColorandOpacity (Variables|Default|GetWidget) "(R=0.000000,G=0.384457,B=1.000000,A=1.000000)")))))

(fn RemoveRoad
  (if (Utilities|Enum|Equal(Enum) (Utilities|Struct|BreakS_TileData (Variables|Default|GetTile%20Data)) "NewEnumerator1")
    (Components|StaticMesh|SetStaticMesh (Variables|Default|GetHex) "/Game/Assets/Tiles/Base/SM_hex_grass.SM_hex_grass")
    (Utilities|Struct|SetmembersinS_TileData (Variables|Default|GetTile%20Data) "NewEnumerator0" false)))

(fn AdjacenttoRoad?
  (bind _tile_neighbour (Variables|Default|GetTile%20Neighbour))
  (bind (_nneighbour _neneighbour _seneighbour _sneighbour _swneighbour _nwneighbour) (Utilities|Struct|BreakS_TileNeighbour _tile_neighbour))
  (for _array_element (Utilities|Array|MakeArray _nneighbour _neneighbour _seneighbour _sneighbour _swneighbour _nwneighbour)
    (Utilities|IsValid _array_element
      (:Is%20Valid
        (if (Utilities|Enum|Equal(Enum) (Utilities|Struct|BreakS_TileData (Variables|BP_HexTile_C|GetTile%20Data _array_element)) "NewEnumerator1")
          (return true)))))
  (return false))

(fn CanPlayerAfford?
  (return false))

(fn GainedBonusResources?
  (return false))

(fn InBuildMode?
  (return false))

(fn InDemoMode?
  (return false))

(fn InRoadMode?
  (return false))

(fn IsAdjacenttoRuleBP?
  (params (Rule%20BPs :type Array%20of%20Actor%20Class%20References))
  (bind _tile_neighbour (Variables|Default|GetTile%20Neighbour))
  (bind (_nneighbour _neneighbour _seneighbour _sneighbour _swneighbour _nwneighbour) (Utilities|Struct|BreakS_TileNeighbour _tile_neighbour))
  (LocalVariables|SetL%20Rule%20BPs Rule%20BPs)
  (for _array_element (Utilities|Array|MakeArray _nneighbour _neneighbour _seneighbour _sneighbour _swneighbour _nwneighbour)
    (Utilities|IsValid _array_element
      (:Is%20Valid
        (if (Utilities|Array|ContainsItem (LocalVariables|GetL%20Rule%20BPs) (Utilities|GetClass (Utilities|Struct|BreakS_TileData (Variables|BP_HexTile_C|GetTile%20Data _array_element))))
          (return true)))))
  (return false))

(fn TileOccupied?
  (return (Utilities|Struct|BreakS_TileData (Variables|Default|GetTile%20Data))))