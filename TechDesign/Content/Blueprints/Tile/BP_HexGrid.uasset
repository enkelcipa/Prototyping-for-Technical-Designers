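; Hex grid generator that spawns BP_HexTile actors on BeginPlay and paints them with four biome types.
; Tiles are stored by coordinate in a map and linked to six neighbours, choosing offsets by array-index parity.
; Perlin noise, randomly offset per tile, seeds biomes, which spread to neighbours in shuffled order.
; Isolated tiles then adopt their commonest neighbouring biome before materials and tile event bindings are set.
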(event EventBeginPlay
  (CallFunction|CreateGrid)
  (NeighbourTiles|GetNeighbourTiles)
  (CallFunction|GenerateNoise)
  (CallFunction|ExpandBiomes)
  (CallFunction|RemoveSoloTiles)
  (CallFunction|AssignBiomeMaterial)
  (bind _values (Utilities|Map|Values (Variables|Default|GetTile%20+%20Coord)))
  (for _array_element _values
    (Default|Init:EventBindings _array_element)))

(fn ConstructionScript)

(fn SpawnTile
  (params (Transform :type Transform))
  (bind _returnvalue (AddComponent|AddChildActorComponent false Transform))
  (ChildActorComponent|SetChildActorClass _returnvalue "/Game/Blueprints/Tile/BP_HexTile.BP_HexTile_C"))

(fn CreateGrid
  (for _index (range 0 (- (Variables|Default|GetColumn%20Length) 1))
    (LocalVariables|SetGrid%20X _index)
    (for _index_2 (range 0 (- (Variables|Default|GetRow%20Length) 1))
      (LocalVariables|SetGrid%20Y _index_2)
      (bind _returnvalue (Game|SpawnActorfromClass "/Game/Blueprints/Tile/BP_HexTile.BP_HexTile_C" (Math|Transform|MakeTransform (Math|Vector|SelectVector (Math|Vector|MakeVector (* _index (|(Radius*SQRT) 115.0 (Math|Float|Sqrt 3.0))) (* _index_2 (|((Radius*2)*0.750000) 115.0)) 15.0) (Math|Vector|MakeVector (+ (|((Radius*SQRT)/2) 115.0 (Math|Float|Sqrt 3.0)) (* _index (|(Radius*SQRT) 115.0 (Math|Float|Sqrt 3.0)))) (* _index_2 (|((Radius*2)*0.750000) 115.0)) 15.0) (== (Math|Integer|%(Integer) _index_2 2) 0))) "Undefined" "MultiplyWithRoot" 0 0))
      (Utilities|Struct|SetmembersinS_TileData (Variables|/Game/Blueprints/Tile/BP_HexTile.BP_HexTile_C|GetTile%20Data _returnvalue) (Math|Vector2D|MakeVector2D (Math|Conversions|ToFloat(Integer) (LocalVariables|GetGrid%20X)) (Math|Conversions|ToFloat(Integer) (LocalVariables|GetGrid%20Y))))
      (Utilities|Map|Add (Variables|Default|GetTile%20+%20Coord) (Math|Vector2D|MakeVector2D (Math|Conversions|ToFloat(Integer) (LocalVariables|GetGrid%20X)) (Math|Conversions|ToFloat(Integer) (LocalVariables|GetGrid%20Y))) _returnvalue))))

(fn GetNeighbourTiles
  (bind _values (Utilities|Map|Values (Variables|Default|GetTile%20+%20Coord)))
  (for (_array_element _array_index) _values
    (LocalVariables|SetL%20Current%20Tile _array_element)
    (if (or (== (Math|Integer|%(Integer) _array_index 2) 0) (== _array_index 0))
      (NeighbourTiles|EvenNeighbourTiles (LocalVariables|GetL%20Current%20Tile))
      (else
        (NeighbourTiles|OddNeighbourTiles (LocalVariables|GetL%20Current%20Tile))))))

(fn GenerateNoise
  (bind _values (Utilities|Map|Values (Variables|Default|GetTile%20+%20Coord)))
  (for _array_element _values
    (LocalVariables|SetL%20Current%20Tile _array_element)
    (LocalVariables|SetL%20BiomeNoiseOffsetX (Math|Random|RandomFloatinRange 0.0 1e+03))
    (LocalVariables|SetL%20BiomeNoiseOffsetY (Math|Random|RandomFloatinRange 0.0 1e+03))
    (bind _biome_type (CallFunction|SelectBiomeType (Class|KismetAnimationLibrary|MakePerlinNoiseandRemap (+ (|((Grid*NoiseScale)+Offset) (.X (Math|Vector2D|BreakVector2D (.TileCoordinate (Utilities|Struct|BreakS_TileData (Variables|/Game/Blueprints/Tile/BP_HexTile.BP_HexTile_C|GetTile%20Data _array_element))))) (LocalVariables|GetL%20BiomeNoiseOffsetX) (LocalVariables|GetL%20BiomeNoiseScale)) (|((Grid*NoiseScale)+Offset) (.Y (Math|Vector2D|BreakVector2D (.TileCoordinate (Utilities|Struct|BreakS_TileData (Variables|/Game/Blueprints/Tile/BP_HexTile.BP_HexTile_C|GetTile%20Data _array_element))))) (LocalVariables|GetL%20BiomeNoiseOffsetY) (LocalVariables|GetL%20BiomeNoiseScale))) 0.0 1.0)))
    (Utilities|Struct|SetmembersinS_TileData (Variables|/Game/Blueprints/Tile/BP_HexTile.BP_HexTile_C|GetTile%20Data (LocalVariables|GetL%20Current%20Tile)) _biome_type)))

(fn SelectBiomeType
  (params (Noise%20Value :type Float%20%28double-precision%29))
  (bind _output_get (LocalVariables|SetL%20Noise%20Value Noise%20Value))
  (if (<= _output_get 0.3)
    (return "NewEnumerator0")
    (elif (<= (LocalVariables|GetL%20Noise%20Value) 0.55)
      (return "NewEnumerator1")
      (elif (<= (LocalVariables|GetL%20Noise%20Value) 0.8)
        (return "NewEnumerator2")
        (else
          (return "NewEnumerator3"))))))

(fn AssignBiomeMaterial
  (bind _values (Utilities|Map|Values (Variables|Default|GetTile%20+%20Coord)))
  (for _array_element _values
    (Rendering|Material|SetMaterial (Variables|/Game/Blueprints/Tile/BP_HexTile.BP_HexTile_C|GetHex _array_element) 0 (.Value (Utilities|Map|Find (LocalVariables|GetL%20Biome%20Material) (Utilities|Struct|BreakS_TileData (Variables|/Game/Blueprints/Tile/BP_HexTile.BP_HexTile_C|GetTile%20Data _array_element)))))))

(fn EvenNeighbourTiles
  (params (Current%20Tile :type BP%20Hex%20Tile%20Object%20Reference))
  (bind _tile_data (Variables|/Game/Blueprints/Tile/BP_HexTile.BP_HexTile_C|GetTile%20Data Current%20Tile))
  (bind _tilecoordinate (Utilities|Struct|BreakS_TileData _tile_data))
  (Utilities|Struct|SetmembersinS_TileNeighbour (Variables|/Game/Blueprints/Tile/BP_HexTile.BP_HexTile_C|GetTile%20Neighbour Current%20Tile) (NeighbourTiles|NNeighbour _tilecoordinate) (NeighbourTiles|EvenNE+OddSENeighbour _tilecoordinate) (NeighbourTiles|EvenSENeighbour _tilecoordinate) (NeighbourTiles|SNeighbour _tilecoordinate) (NeighbourTiles|EvenSWNeighbour _tilecoordinate) (NeighbourTiles|EvenNW+OddSWNeighbour _tilecoordinate)))

(fn OddNeighbourTiles
  (params (Current%20Tile :type BP%20Hex%20Tile%20Object%20Reference))
  (bind _tile_data (Variables|/Game/Blueprints/Tile/BP_HexTile.BP_HexTile_C|GetTile%20Data Current%20Tile))
  (bind _tilecoordinate (Utilities|Struct|BreakS_TileData _tile_data))
  (Utilities|Struct|SetmembersinS_TileNeighbour (Variables|/Game/Blueprints/Tile/BP_HexTile.BP_HexTile_C|GetTile%20Neighbour Current%20Tile) (NeighbourTiles|NNeighbour _tilecoordinate) (NeighbourTiles|OddNENeighbour _tilecoordinate) (NeighbourTiles|EvenNE+OddSENeighbour _tilecoordinate) (NeighbourTiles|SNeighbour _tilecoordinate) (NeighbourTiles|EvenNW+OddSWNeighbour _tilecoordinate) (NeighbourTiles|OddNWNeighbour _tilecoordinate)))

(fn NNeighbour
  (params (Coordinates :type Vector%202D%20Structure))
  (bind (_x _y) (Math|Vector2D|BreakVector2D Coordinates))
  (return (.Value (Utilities|Map|Find (Variables|Default|GetTile%20+%20Coord) (Math|Vector2D|MakeVector2D (+ _x 1.0) _y)))))

(fn SNeighbour
  (params (Coordinates :type Vector%202D%20Structure))
  (bind (_x _y) (Math|Vector2D|BreakVector2D Coordinates))
  (return (.Value (Utilities|Map|Find (Variables|Default|GetTile%20+%20Coord) (Math|Vector2D|MakeVector2D (- _x 1.0) _y)))))

(fn EvenNE+OddSENeighbour
  (params (Coordinates :type Vector%202D%20Structure))
  (bind (_x _y) (Math|Vector2D|BreakVector2D Coordinates))
  (return (.Value (Utilities|Map|Find (Variables|Default|GetTile%20+%20Coord) (Math|Vector2D|MakeVector2D _x (+ _y 1.0))))))

(fn EvenSENeighbour
  (params (Coordinates :type Vector%202D%20Structure))
  (bind (_x _y) (Math|Vector2D|BreakVector2D Coordinates))
  (return (.Value (Utilities|Map|Find (Variables|Default|GetTile%20+%20Coord) (Math|Vector2D|MakeVector2D (- _x 1.0) (+ _y 1.0))))))

(fn EvenSWNeighbour
  (params (Coordinates :type Vector%202D%20Structure))
  (bind (_x _y) (Math|Vector2D|BreakVector2D Coordinates))
  (return (.Value (Utilities|Map|Find (Variables|Default|GetTile%20+%20Coord) (Math|Vector2D|MakeVector2D (- _x 1.0) (- _y 1.0))))))

(fn EvenNW+OddSWNeighbour
  (params (Coordinates :type Vector%202D%20Structure))
  (bind (_x _y) (Math|Vector2D|BreakVector2D Coordinates))
  (return (.Value (Utilities|Map|Find (Variables|Default|GetTile%20+%20Coord) (Math|Vector2D|MakeVector2D _x (- _y 1.0))))))

(fn OddNENeighbour
  (params (Coordinates :type Vector%202D%20Structure))
  (bind (_x _y) (Math|Vector2D|BreakVector2D Coordinates))
  (return (.Value (Utilities|Map|Find (Variables|Default|GetTile%20+%20Coord) (Math|Vector2D|MakeVector2D (+ _x 1.0) (+ _y 1.0))))))

(fn OddNWNeighbour
  (params (Coordinates :type Vector%202D%20Structure))
  (bind (_x _y) (Math|Vector2D|BreakVector2D Coordinates))
  (return (.Value (Utilities|Map|Find (Variables|Default|GetTile%20+%20Coord) (Math|Vector2D|MakeVector2D (+ _x 1.0) (- _y 1.0))))))

(fn ExpandBiomes
  (bind _values (Utilities|Map|Values (Variables|Default|GetTile%20+%20Coord)))
  (bind _output_get (LocalVariables|SetL%20Tile%20Grid _values))
  (Utilities|Array|Shuffle _output_get)
  (for _array_element (LocalVariables|GetL%20Tile%20Grid)
    (Utilities|IsValid _array_element
      (:Is%20Valid
        (LocalVariables|SetL%20Tile%20Biome (.Biome (Utilities|Struct|BreakS_TileData (Variables|/Game/Blueprints/Tile/BP_HexTile.BP_HexTile_C|GetTile%20Data _array_element))))
        (for _array_element_2 (Utilities|Array|MakeArray (.NNeighbour (Utilities|Struct|BreakS_TileNeighbour (Variables|/Game/Blueprints/Tile/BP_HexTile.BP_HexTile_C|GetTile%20Neighbour _array_element))) (.NENeighbour (Utilities|Struct|BreakS_TileNeighbour (Variables|/Game/Blueprints/Tile/BP_HexTile.BP_HexTile_C|GetTile%20Neighbour _array_element))) (.SENeighbour (Utilities|Struct|BreakS_TileNeighbour (Variables|/Game/Blueprints/Tile/BP_HexTile.BP_HexTile_C|GetTile%20Neighbour _array_element))) (.SNeighbour (Utilities|Struct|BreakS_TileNeighbour (Variables|/Game/Blueprints/Tile/BP_HexTile.BP_HexTile_C|GetTile%20Neighbour _array_element))) (.SWNeighbour (Utilities|Struct|BreakS_TileNeighbour (Variables|/Game/Blueprints/Tile/BP_HexTile.BP_HexTile_C|GetTile%20Neighbour _array_element))) (.NWNeighbour (Utilities|Struct|BreakS_TileNeighbour (Variables|/Game/Blueprints/Tile/BP_HexTile.BP_HexTile_C|GetTile%20Neighbour _array_element))))
          (Utilities|IsValid _array_element_2
            (:Is%20Valid
              (Utilities|Struct|SetmembersinS_TileData (Variables|/Game/Blueprints/Tile/BP_HexTile.BP_HexTile_C|GetTile%20Data _array_element_2) (LocalVariables|GetL%20Tile%20Biome)))))))))

(fn RemoveSoloTiles
  (Utilities|Set|Clear (LocalVariables|GetL%20Solo%20Tiles))
  (bind _values (Utilities|Map|Values (Variables|Default|GetTile%20+%20Coord)))
  (for _array_element _values
    (LocalVariables|SetL%20Current%20Tile _array_element)
    (LocalVariables|SetL%20Solo%20Tile? true)
    (bind _array_element_2 (Utilities|Array|ForEachLoopwithBreak (Utilities|Array|MakeArray (.NNeighbour (Utilities|Struct|BreakS_TileNeighbour (Variables|/Game/Blueprints/Tile/BP_HexTile.BP_HexTile_C|GetTile%20Neighbour _array_element))) (.NENeighbour (Utilities|Struct|BreakS_TileNeighbour (Variables|/Game/Blueprints/Tile/BP_HexTile.BP_HexTile_C|GetTile%20Neighbour _array_element))) (.SENeighbour (Utilities|Struct|BreakS_TileNeighbour (Variables|/Game/Blueprints/Tile/BP_HexTile.BP_HexTile_C|GetTile%20Neighbour _array_element))) (.SNeighbour (Utilities|Struct|BreakS_TileNeighbour (Variables|/Game/Blueprints/Tile/BP_HexTile.BP_HexTile_C|GetTile%20Neighbour _array_element))) (.SWNeighbour (Utilities|Struct|BreakS_TileNeighbour (Variables|/Game/Blueprints/Tile/BP_HexTile.BP_HexTile_C|GetTile%20Neighbour _array_element))) (.NWNeighbour (Utilities|Struct|BreakS_TileNeighbour (Variables|/Game/Blueprints/Tile/BP_HexTile.BP_HexTile_C|GetTile%20Neighbour _array_element)))) :!label _label)
      (:LoopBody
        (Utilities|IsValid _array_element_2
          (:Is%20Valid
            (if (Utilities|Enum|Equal(Enum) (.Biome (Utilities|Struct|BreakS_TileData (Variables|/Game/Blueprints/Tile/BP_HexTile.BP_HexTile_C|GetTile%20Data _array_element_2))) (.Biome (Utilities|Struct|BreakS_TileData (Variables|/Game/Blueprints/Tile/BP_HexTile.BP_HexTile_C|GetTile%20Data (LocalVariables|GetL%20Current%20Tile)))))
              (LocalVariables|SetL%20Solo%20Tile? false)
              (goto _label Break)))))
      (:Completed
        (if (LocalVariables|GetL%20Solo%20Tile?)
          (Utilities|Set|Add (LocalVariables|GetL%20Solo%20Tiles) (LocalVariables|GetL%20Current%20Tile))))))
  (bind _valuepin (Utilities|Set|ForEachLoop(Set) (LocalVariables|GetL%20Solo%20Tiles))
    (:then
      (LocalVariables|SetL%20Biome%20Count (Utilities|Map|MakeMap "NewEnumerator0" 0 "NewEnumerator1" 0 "NewEnumerator2" 0 "NewEnumerator3" 0))
      (LocalVariables|SetL%20Current%20Tile _valuepin)
      (LocalVariables|SetL%20Highest%20Count 0)
      (for _array_element_3 (Utilities|Array|MakeArray (.NNeighbour (Utilities|Struct|BreakS_TileNeighbour (Variables|/Game/Blueprints/Tile/BP_HexTile.BP_HexTile_C|GetTile%20Neighbour _valuepin))) (.NENeighbour (Utilities|Struct|BreakS_TileNeighbour (Variables|/Game/Blueprints/Tile/BP_HexTile.BP_HexTile_C|GetTile%20Neighbour _valuepin))) (.SENeighbour (Utilities|Struct|BreakS_TileNeighbour (Variables|/Game/Blueprints/Tile/BP_HexTile.BP_HexTile_C|GetTile%20Neighbour _valuepin))) (.SNeighbour (Utilities|Struct|BreakS_TileNeighbour (Variables|/Game/Blueprints/Tile/BP_HexTile.BP_HexTile_C|GetTile%20Neighbour _valuepin))) (.SWNeighbour (Utilities|Struct|BreakS_TileNeighbour (Variables|/Game/Blueprints/Tile/BP_HexTile.BP_HexTile_C|GetTile%20Neighbour _valuepin))) (.NWNeighbour (Utilities|Struct|BreakS_TileNeighbour (Variables|/Game/Blueprints/Tile/BP_HexTile.BP_HexTile_C|GetTile%20Neighbour _valuepin))))
        (Utilities|IsValid _array_element_3
          (:Is%20Valid
            (Utilities|Map|Add (LocalVariables|GetL%20Biome%20Count) (.Biome (Utilities|Struct|BreakS_TileData (Variables|/Game/Blueprints/Tile/BP_HexTile.BP_HexTile_C|GetTile%20Data _array_element_3))) (+ (.Value (Utilities|Map|Find (LocalVariables|GetL%20Biome%20Count) (.Biome (Utilities|Struct|BreakS_TileData (Variables|/Game/Blueprints/Tile/BP_HexTile.BP_HexTile_C|GetTile%20Data _array_element_3))))) 1)))))
      (bind (_keypin _valuepin_2) (Utilities|Map|ForEachLoop(Map) (LocalVariables|GetL%20Biome%20Count))
        (:then
          (if (> _valuepin_2 (LocalVariables|GetL%20Highest%20Count))
            (LocalVariables|SetL%20Biome%20to%20Change%20to _keypin)
            (LocalVariables|SetL%20Highest%20Count _valuepin_2)))
        (:CompletedPin
          (Utilities|Struct|SetmembersinS_TileData (Variables|/Game/Blueprints/Tile/BP_HexTile.BP_HexTile_C|GetTile%20Data (LocalVariables|GetL%20Current%20Tile)) (LocalVariables|GetL%20Biome%20to%20Change%20to)))))))