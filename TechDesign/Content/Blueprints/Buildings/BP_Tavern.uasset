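; BP_Tavern is a child building that generates citizens and population, with gold output and upkeep that grow with them.
; On each GenerateResource, it adds one citizen and population through the GameMode until it reaches its cap, then runs the parent logic.
; Each new citizen rebuilds the gold production map and food and firewood cost maps in BuildingData.
; Refunding also removes the citizens and population it generated.
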(event Custom|Update%20Production%20and%20Consumption
  (bind _returnvalue (Game|GetGameMode))
  (bind _building_data (Variables|Default|GetBuilding%20Data))
  (bind _building_data_2 (Variables|Default|GetBuilding%20Data))
  (bind _citizensgenerated (Utilities|Struct|BreakS_BuildingData _building_data))
  (bind (_citizensgenerated_2 _goldpercitizen) (Utilities|Struct|BreakS_BuildingData _building_data_2))
  ;[0.15 0.15 0.15 0.5] Generate 1 Citizen and Population
  (Math|Float|IncrementFloat _citizensgenerated_2
    (:%20%20
      (Class|BPIResources|UpdateResources(Message) _returnvalue "NewEnumerator15" 1.0 false)
      (Class|BPIResources|UpdateResources(Message) _returnvalue "NewEnumerator0" 1.0 false)
      ;[0.15 0.15 0.15 0.5] Update Gold Generated
      (Utilities|Struct|SetmembersinS_BuildingData (Variables|Default|GetBuilding%20Data) (Utilities|Map|MakeMap "NewEnumerator2" (* _citizensgenerated_2 _goldpercitizen)))
      ;[0.15 0.15 0.15 0.5] Update Food and Firewood Costs
      (Utilities|Struct|SetmembersinS_BuildingData (Variables|Default|GetBuilding%20Data) (Utilities|Map|MakeMap "NewEnumerator1" (* _citizensgenerated 15.0) "NewEnumerator5" (* _citizensgenerated 1e+01))))))

(event EventGenerateResource
  (bind _building_data (Variables|Default|GetBuilding%20Data))
  (bind (_citizensgenerated _maxcitizengen) (Utilities|Struct|BreakS_BuildingData _building_data))
  ;[0.15 0.15 0.15 0.5] Check if Tavern can generate a new Citizen and Population
  (if (< _citizensgenerated _maxcitizengen)
    ;[0.15 0.15 0.15 0.5] Update Production and Consumption Maps if True
    (CallFunction|UpdateProductionandConsumption))
  (|CallParentFunction))

(fn ConstructionScript
  (|CallParentFunction))

(fn RefundResources
  (bind _returnvalue (Game|GetGameMode))
  (bind _building_data (Variables|Default|GetBuilding%20Data))
  (bind _citizensgenerated (Utilities|Struct|BreakS_BuildingData _building_data))
  (|CallParentFunction)
  (Class|BPIResources|UpdateResources(Message) _returnvalue "NewEnumerator0" _citizensgenerated true)
  (Class|BPIResources|UpdateResources(Message) _returnvalue "NewEnumerator15" _citizensgenerated true))