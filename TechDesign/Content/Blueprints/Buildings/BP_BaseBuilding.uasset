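; Base class for placeable, resource-producing buildings in a tile-based builder, covering placement preview, economy and demolition.
; A looping timer drives the cursor-following preview, which snaps to tiles and turns green or red based on occupancy, build mode, cost and road, neighbour or uniqueness rules.
; Placing occupies the tile and charges costs, resource ticks exchange inputs for outputs, and removal refunds costs.
; Game mode and tiles are reached through interface messages.
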(event OnClicked(BuildingMesh)
  (params (TouchedComponent :type Primitive%20Component%20Object%20Reference) (ButtonPressed :type Key%20Structure :default "None"))
  (if (not (CallFunction|PlayerinDemoMode?))
    (Class|BPISetters|SetSelectedBuilding(Message) (Game|GetGameMode) self)
    (Class|BPIUI|ToggleDetailsPanel(Message) (Game|GetGameMode) true (Variables|Default|GetBuilding%20Data))))

(event OnBeginCursorOver(BuildingMesh)
  (params (TouchedComponent :type Primitive%20Component%20Object%20Reference))
  (Class|BPIUI|ToggleTileOverlay(Message) (Utilities|Struct|BreakS_BuildingData (Variables|Default|GetBuilding%20Data)) true))

(event OnEndCursorOver(BuildingMesh)
  (params (TouchedComponent :type Primitive%20Component%20Object%20Reference))
  (Class|BPIUI|ToggleTileOverlay(Message) (Utilities|Struct|BreakS_BuildingData (Variables|Default|GetBuilding%20Data)) false)
  (if (CallFunction|PlayerinDemoMode?)
    (CallFunction|PlacedMaterial)
    (CallFunction|ToggleBuildingCollisions true)))

(event Custom|Placement%20Mode
  ;[0.15 0.15 0.15 0.5] Used for updating location of the object
  (bind _returnvalue (Utilities|Time|SetTimerbyEvent (EventDispatchers|CreateEvent :!event UpdateLocation) 0.1 true))
  (Variables|Default|SetPlacment%20Timer _returnvalue))

(event Custom|Placed%20Material
  ;[0.15 0.15 0.15 0.5] Placement Materials
  (for _array_element (Variables|Default|GetMeshes)
    (Rendering|Material|SetMaterial _array_element 0 "/Game/Assets/Materials/M_Buildings.M_Buildings")))

(event Custom|Generate%20Resource
  (bind (_keypin _valuepin) (Utilities|Map|ForEachLoop(Map) (Utilities|Struct|BreakS_BuildingData (Variables|Default|GetBuilding%20Data)))
    (:then
      (Class|BPIResources|UpdateResources(Message) (Game|GetGameMode) _keypin _valuepin false))))

(event Custom|Valid%20Placement
  ;[0.15 0.15 0.15 0.5] Placement Materials
  (for _array_element (Variables|Default|GetMeshes)
    (Rendering|Material|SetMaterial _array_element 0 "/Game/Assets/Materials/MI_PlacementGreen.MI_PlacementGreen")))

(event Custom|Consume%20Resource
  (bind (_keypin _valuepin) (Utilities|Map|ForEachLoop(Map) (Utilities|Struct|BreakS_BuildingData (Variables|Default|GetBuilding%20Data)))
    (:then
      (Class|BPIResources|UpdateResources(Message) (Game|GetGameMode) _keypin _valuepin true))))

(event Custom|Invalid%20Placement
  ;[0.15 0.15 0.15 0.5] Placement Materials
  (for _array_element (Variables|Default|GetMeshes)
    (Rendering|Material|SetMaterial _array_element 0 "/Game/Assets/Materials/MI_PlacementRed.MI_PlacementRed")))

(event EventBeginPlay
  (Variables|Default|SetMeshes (Utilities|Array|MakeArray (Variables|Default|GetBuilding%20Mesh)))
  (CallFunction|InvalidPlacement)
  (CallFunction|PlacementMode))

(event EventPlaceBuilding
  (params (Tile :type Actor%20Object%20Reference))
  (Class|BPISetters|UpdateTileData(Message) Tile true self)
  (Utilities|Struct|SetmembersinS_BuildingData (Variables|Default|GetBuilding%20Data) Tile self)
  (Utilities|Time|ClearandInvalidateTimerbyHandle (Variables|Default|GetPlacment%20Timer))
  (bind _placement_location (CallFunction|GetPlacementLocation))
  (Transformation|SetActorLocation _placement_location false false)
  (CallFunction|PlacedMaterial)
  (CallFunction|ToggleBuildingCollisions true)
  (bind (_keypin _valuepin) (Utilities|Map|ForEachLoop(Map) (Utilities|Struct|BreakS_BuildingData (Variables|Default|GetBuilding%20Data)))
    (:then
      (Class|BPIResources|UpdateResources(Message) (Game|GetGameMode) _keypin _valuepin true))))

(event EventTickResources
  (if (CallFunction|EnoughResources?)
    (CallFunction|GenerateResource)
    (CallFunction|ConsumeResource)
    (else
      (Development|PrintString "Not enough resources"))))

(event EventDemolitionPreview
  (params (Preview? :type Boolean))
  ;[0.15 0.15 0.15 0.5] Demolition Preview Material
  (if Preview?
    (for _array_element (Variables|Default|GetMeshes)
      (Rendering|Material|SetMaterial _array_element 0 "/Game/Assets/Materials/MI_Demolition.MI_Demolition"))
    (else
      (CallFunction|PlacedMaterial))))

(event EventRemoveBuilding
  (params (Building%20to%20Remove :type Actor%20Object%20Reference))
  (bind _returnvalue (Game|GetGameMode))
  (Class|BPIBuild|RemoveBuilding(Message) _returnvalue self)
  (Class|BPIUI|ToggleDetailsPanel(Message) _returnvalue false)
  (CallFunction|RefundResources)
  (Actor|DestroyActor))

(event EventToggleBuildingCollisions
  (params (Enabled? :type Boolean))
  ;[0.15 0.15 0.15 0.5] Building Collisions
  (for _array_element (Variables|Default|GetMeshes)
    (Collision|SetCollisionResponsetoAllChannels _array_element (select Enabled? "ECR_Block" "ECR_Ignore"))))

(fn ConstructionScript)

(fn UpdateLocation
  (bind _returnvalue (Game|GetGameMode))
  (bind _returnvalue_2 (Game|GetPlayerController 0))
  (bind _returnvalue_3 (Game|GetPlayerController 0))
  (bind _returnvalue_4 (Game|GetPlayerController 0))
  (bind _hitresult (Game|Player|GetHitResultUnderCursorbyChannel _returnvalue_2 "TraceTypeQuery1" true))
  (bind _worldlocation (Game|Player|ConvertMouseLocationToWorldSpace _returnvalue_4))
  (bind _hitresult_2 (Game|Player|GetHitResultUnderCursorbyChannel _returnvalue_3 "TraceTypeQuery1" true))
  (bind _hitactor (Collision|BreakHitResult _hitresult))
  (bind _hitactor_2 (Collision|BreakHitResult _hitresult_2))
  (Utilities|IsValid _hitactor_2
    (:Is%20Valid
      (if (Actor|ActorHasTag _hitactor_2 "Tile")
        (Transformation|SetActorLocation (Transformation|GetActorLocation _hitactor_2) false false)
        (bind _rules_followed_ (CallFunction|RulesFollowed? _hitactor))
        (bind _is_occupied_ (Class|BPIQuery|TileOccupied?(Message) _hitactor))
        (bind _in_build_mode_ (Class|BPIQuery|InBuildMode?(Message) _returnvalue))
        (bind _can_afford_ (Class|BPIQuery|CanPlayerAfford?(Message) _returnvalue))
        (if (Math|Boolean|ANDBoolean _can_afford_ _in_build_mode_ (not _is_occupied_) _rules_followed_)
          (CallFunction|ValidPlacement)
          (else
            (CallFunction|InvalidPlacement)))))
    (:Is%20Not%20Valid
      (Transformation|SetActorLocation (Math|Vector|MakeVector (.x _worldlocation) (.y _worldlocation) 15.0) false false))))

(fn GetPlacementLocation
  (bind _returnvalue (Game|GetPlayerController 0))
  (bind _hitresult (Game|Player|GetHitResultUnderCursorbyChannel _returnvalue "TraceTypeQuery1" true))
  (bind _hitactor (Collision|BreakHitResult _hitresult))
  (Utilities|IsValid _hitactor
    (:Is%20Valid
      (if (Actor|ActorHasTag _hitactor "Tile")
        (return (Transformation|GetActorLocation _hitactor))))))

(fn CanAfford?
  (LocalVariables|SetWithin%20Budget? true)
  (bind (_keypin _valuepin) (Utilities|Map|ForEachLoop(Map) (.PlacementCost (Utilities|Struct|BreakS_BuildingData (Variables|Default|GetBuilding%20Data))) :!label _label)
    (:then
      (bind _amount_found (Class|BPIGetters|GetResourceAmount(Message) (Game|GetGameMode) _keypin))
      (if (not (>= _amount_found _valuepin))
        (LocalVariables|SetWithin%20Budget? false)
        (goto _label BreakPin)))
    (:CompletedPin
      (return (LocalVariables|GetWithin%20Budget?)))))

(fn RulesFollowed?
  (params (Tile :type Actor%20Object%20Reference))
  (LocalVariables|SetL%20Tile Tile)
  (LocalVariables|SetL%20Rules true)
  (for _array_element (Utilities|Struct|BreakS_BuildingData (Variables|Default|GetBuilding%20Data))
    (switch Utilities|FlowControl|Switch|SwitchonE_PlacementRule _array_element
      (:NewEnumerator0
        (bind _road_adjacent_ (Class|BPIQuery|AdjacenttoRoad?(Message) (LocalVariables|GetL%20Tile)))
        (if (not _road_adjacent_)
          (LocalVariables|SetL%20Rules false :!label _label)))
      (:NewEnumerator2
        (bind _bp_adjacent_ (Class|BPIQuery|IsAdjacenttoRuleBP?(Message) (LocalVariables|GetL%20Tile) (Utilities|Struct|BreakS_BuildingData (Variables|Default|GetBuilding%20Data))))
        (if (not _bp_adjacent_)
          (goto _label)))
      (:NewEnumerator1
        (bind _placed_buildings (Class|BPIGetters|GetPlacedBuildingsArray(Message) (Game|GetGameMode)))
        (for _array_element_2 _placed_buildings
          (if (== (Utilities|GetClass _array_element_2) (Utilities|GetClass self))
            (goto _label))))))
  (return (LocalVariables|GetL%20Rules)))

(fn EnoughResources?
  (bind (_keypin _valuepin) (Utilities|Map|ForEachLoop(Map) (Utilities|Struct|BreakS_BuildingData (Variables|Default|GetBuilding%20Data)))
    (:then
      (bind _amount_found (Class|BPIGetters|GetResourceAmount(Message) (Game|GetGameMode) _keypin))
      (if (< _amount_found _valuepin)
        (return false)))
    (:CompletedPin
      (return true))))

(fn RefundResources
  (bind (_keypin _valuepin) (Utilities|Map|ForEachLoop(Map) (Utilities|Struct|BreakS_BuildingData (Variables|Default|GetBuilding%20Data)))
    (:then
      (Class|BPIResources|UpdateResources(Message) (Game|GetGameMode) _keypin _valuepin false))))

(fn AdjacenttoRoad?
  (return false))

(fn CanPlayerAfford?
  (bind _can_afford_ (CallFunction|CanAfford?))
  (return _can_afford_))

(fn GetAttachedActors
  (return 0))

(fn GetCurrentBuildingtoPlace
  (return 0))

(fn GetPlacedBuildingsArray
  (return 0))

(fn GetPlacementRules
  (bind _building_data (Variables|Default|GetBuilding%20Data))
  (bind (_placementrule _prulebp) (Utilities|Struct|BreakS_BuildingData _building_data))
  (return _placementrule _prulebp))

(fn GetResourceAmount
  (params (Resource%20to%20Find :type E_Resources%20Enum :default "NewEnumerator15"))
  (return 0.0))

(fn GetSelectedBuildingData
  (return ""))

(fn InBuildMode?
  (return false))

(fn InDemoMode?
  (return false))

(fn InRoadMode?
  (return false))

(fn IsAdjacenttoRuleBP?
  (params (Rule%20BPs :type Array%20of%20Actor%20Class%20References))
  (return false))

(fn TileOccupied?
  (return false))