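; BP_Market is a building Blueprint for the market, which generates income in proportion to the population.
; It overrides GenerateResource, calling the parent first, then reads a resource amount (apparently citizens) from the Game Mode.
; That amount is multiplied by GoldPerCitizen from BuildingData and added to another resource, presumably gold, through Game Mode interface messages.
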(event EventBeginPlay
  (|CallParentFunction))

(event Collision|EventActorBeginOverlap
  (params (OtherActor :type Actor%20Object%20Reference))
  (|CallParentFunction OtherActor) ; This node is disabled and will not be called.\nDrag off pins to build functionality.
)

(event EventTick
  (params (DeltaSeconds :type Float%20%28single-precision%29))
  (|CallParentFunction DeltaSeconds) ; This node is disabled and will not be called.\nDrag off pins to build functionality.
)

(event EventGenerateResource
  (|CallParentFunction)
  (bind _amount_found (Class|BPIGetters|GetResourceAmount(Message) (Game|GetGameMode) "NewEnumerator0"))
  (Class|BPIResources|UpdateResources(Message) (Game|GetGameMode) "NewEnumerator2" (* _amount_found (Utilities|Struct|BreakS_BuildingData (Variables|Default|GetBuilding%20Data))) false))

(fn ConstructionScript
  (|CallParentFunction))