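; BP_Lumbermill is a lumbermill building that extends a parent building class with two additional static meshes.
; On BeginPlay it registers them alongside BuildingMesh in the Meshes array.
; Both extra meshes share cursor handlers: clicking opens the details panel and selects the building, while hovering toggles the referenced tile's overlay.
; In demo mode, both hover start and end apply the placed material and enable building collisions.
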(event OnBeginCursorOver(StaticMesh)
  (params (TouchedComponent :type Primitive%20Component%20Object%20Reference))
  ;[0.15 0.15 0.15 0.5] Mouse Events for additional meshes on building
  (Class|BPIUI|ToggleTileOverlay(Message) (Utilities|Struct|BreakS_BuildingData (Variables|Default|GetBuilding%20Data)) true)
  (if (CallFunction|PlayerinDemoMode?)
    (CallFunction|PlacedMaterial)
    (CallFunction|ToggleBuildingCollisions true)))

(event OnEndCursorOver(StaticMesh)
  (params (TouchedComponent :type Primitive%20Component%20Object%20Reference))
  ;[0.15 0.15 0.15 0.5] Mouse Events for additional meshes on building
  (Class|BPIUI|ToggleTileOverlay(Message) (Utilities|Struct|BreakS_BuildingData (Variables|Default|GetBuilding%20Data)) false)
  (if (CallFunction|PlayerinDemoMode?)
    (CallFunction|PlacedMaterial)
    (CallFunction|ToggleBuildingCollisions true)))

(event OnBeginCursorOver(StaticMesh1)
  (params (TouchedComponent :type Primitive%20Component%20Object%20Reference))
  ;[0.15 0.15 0.15 0.5] Mouse Events for additional meshes on building
  (Class|BPIUI|ToggleTileOverlay(Message) (Utilities|Struct|BreakS_BuildingData (Variables|Default|GetBuilding%20Data)) true)
  (if (CallFunction|PlayerinDemoMode?)
    (CallFunction|PlacedMaterial)
    (CallFunction|ToggleBuildingCollisions true)))

(event OnEndCursorOver(StaticMesh1)
  (params (TouchedComponent :type Primitive%20Component%20Object%20Reference))
  ;[0.15 0.15 0.15 0.5] Mouse Events for additional meshes on building
  (Class|BPIUI|ToggleTileOverlay(Message) (Utilities|Struct|BreakS_BuildingData (Variables|Default|GetBuilding%20Data)) false)
  (if (CallFunction|PlayerinDemoMode?)
    (CallFunction|PlacedMaterial)
    (CallFunction|ToggleBuildingCollisions true)))

(event OnClicked(StaticMesh)
  (params (TouchedComponent :type Primitive%20Component%20Object%20Reference) (ButtonPressed :type Key%20Structure))
  ;[0.15 0.15 0.15 0.5] Mouse Events for additional meshes on building
  (Class|BPIUI|ToggleDetailsPanel(Message) (Game|GetGameMode) true (Variables|Default|GetBuilding%20Data))
  (Class|BPISetters|SetSelectedBuilding(Message) (Game|GetGameMode) self))

(event OnClicked(StaticMesh1)
  (params (TouchedComponent :type Primitive%20Component%20Object%20Reference) (ButtonPressed :type Key%20Structure))
  ;[0.15 0.15 0.15 0.5] Mouse Events for additional meshes on building
  (Class|BPIUI|ToggleDetailsPanel(Message) (Game|GetGameMode) true (Variables|Default|GetBuilding%20Data))
  (Class|BPISetters|SetSelectedBuilding(Message) (Game|GetGameMode) self))

(event EventBeginPlay
  (|CallParentFunction)
  (Variables|Default|SetMeshes (Utilities|Array|MakeArray (Variables|Default|GetBuilding%20Mesh) (Variables|Default|GetStaticMesh) (Variables|Default|GetStaticMesh1))))

(event Collision|EventActorBeginOverlap
  (params (OtherActor :type Actor%20Object%20Reference))
  (|CallParentFunction OtherActor) ; This node is disabled and will not be called.\nDrag off pins to build functionality.
)

(event EventTick
  (params (DeltaSeconds :type Float%20%28single-precision%29))
  (|CallParentFunction DeltaSeconds) ; This node is disabled and will not be called.\nDrag off pins to build functionality.
)

(fn ConstructionScript
  (|CallParentFunction))