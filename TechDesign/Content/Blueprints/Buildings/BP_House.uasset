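; BP_House is a house building that generates citizens and turns them into income for the resource economy.
; GenerateResource calls the parent and increments the citizen count until it reaches the cap, then always credits gold scaled by that count.
; ConsumeResource loops over the BuildingData production cost map and deducts each resource multiplied by the citizen count.
; Both events report changes through the game mode's UpdateResourcesMessage.
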(event EventBeginPlay
  (|CallParentFunction))

(event EventGenerateResource
  (bind _building_data (Variables|Default|GetBuilding%20Data))
  (bind _building_data_2 (Variables|Default|GetBuilding%20Data))
  (bind (_citizensgenerated _goldpercitizen) (Utilities|Struct|BreakS_BuildingData _building_data_2))
  (bind (_citizensgenerated_2 _maxcitizengen) (Utilities|Struct|BreakS_BuildingData _building_data))
  (if (< _citizensgenerated_2 _maxcitizengen)
    (|CallParentFunction)
    (Math|Float|IncrementFloat (Utilities|Struct|BreakS_BuildingData (Variables|Default|GetBuilding%20Data))
      (:%20%20
        _)))
  (Class|BPIResources|UpdateResources(Message) (Game|GetGameMode) "NewEnumerator2" (* _citizensgenerated _goldpercitizen) false))

(event EventConsumeResource
  (bind _building_data (Variables|Default|GetBuilding%20Data))
  (bind (_productioncost _citizensgenerated) (Utilities|Struct|BreakS_BuildingData _building_data))
  (bind (_keypin _valuepin) (Utilities|Map|ForEachLoop(Map) _productioncost)
    (:then
      (Class|BPIResources|UpdateResources(Message) (Game|GetGameMode) _keypin (* _valuepin _citizensgenerated) true))))

(fn ConstructionScript
  (|CallParentFunction))