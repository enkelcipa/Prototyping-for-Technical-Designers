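; BP_Windmill is a windmill building, derived from a parent building class, that keeps a list of attached farmland.
; It registers its extra static and blade meshes, mirroring hover and click events to toggle tile overlays, select itself and open the details panel.
; In demo mode, hover changes also apply the placed material and enable collisions.
; Adding farmland refreshes the details widget, and GetAttachedActors returns that list; other getters are stubs.
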(event OnClicked(StaticMesh)
  (params (TouchedComponent :type Primitive%20Component%20Object%20Reference) (ButtonPressed :type Key%20Structure :default "None"))
  ;[0.15 0.15 0.15 0.5] Mouse Events for additional meshes on building
  (Class|BPIUI|ToggleDetailsPanel(Message) (Game|GetGameMode) true (Variables|Default|GetBuilding%20Data))
  (Class|BPISetters|SetSelectedBuilding(Message) (Game|GetGameMode) self))

(event OnClicked(Blade)
  (params (TouchedComponent :type Primitive%20Component%20Object%20Reference) (ButtonPressed :type Key%20Structure :default "None"))
  ;[0.15 0.15 0.15 0.5] Mouse Events for additional meshes on building
  (Class|BPIUI|ToggleDetailsPanel(Message) (Game|GetGameMode) true (Variables|Default|GetBuilding%20Data))
  (Class|BPISetters|SetSelectedBuilding(Message) (Game|GetGameMode) self))

(event OnBeginCursorOver(StaticMesh)
  (params (TouchedComponent :type Primitive%20Component%20Object%20Reference))
  ;[0.15 0.15 0.15 0.5] Mouse Events for additional meshes on building
  (Class|BPIUI|ToggleTileOverlay(Message) (Utilities|Struct|BreakS_BuildingData (Variables|Default|GetBuilding%20Data)) true)
  (if (CallFunction|PlayerinDemoMode?)
    (CallFunction|PlacedMaterial)
    (CallFunction|ToggleBuildingCollisions true)))

(event OnEndCursorOver(StaticMesh)
  (params (TouchedComponent :type Primitive%20Component%20Object%20Reference))
  ;[0.15 0.15 0.15 0.5] Mouse Events for additional meshes on building
  (Class|BPIUI|ToggleTileOverlay(Message) (Utilities|Struct|BreakS_BuildingData (Variables|Default|GetBuilding%20Data)) false)
  (if (CallFunction|PlayerinDemoMode?)
    (CallFunction|PlacedMaterial)
    (CallFunction|ToggleBuildingCollisions true)))

(event OnBeginCursorOver(Blade)
  (params (TouchedComponent :type Primitive%20Component%20Object%20Reference))
  ;[0.15 0.15 0.15 0.5] Mouse Events for additional meshes on building
  (Class|BPIUI|ToggleTileOverlay(Message) (Utilities|Struct|BreakS_BuildingData (Variables|Default|GetBuilding%20Data)) true)
  (if (CallFunction|PlayerinDemoMode?)
    (CallFunction|PlacedMaterial)
    (CallFunction|ToggleBuildingCollisions true)))

(event OnEndCursorOver(Blade)
  (params (TouchedComponent :type Primitive%20Component%20Object%20Reference))
  ;[0.15 0.15 0.15 0.5] Mouse Events for additional meshes on building
  (Class|BPIUI|ToggleTileOverlay(Message) (Utilities|Struct|BreakS_BuildingData (Variables|Default|GetBuilding%20Data)) false)
  (if (CallFunction|PlayerinDemoMode?)
    (CallFunction|PlacedMaterial)
    (CallFunction|ToggleBuildingCollisions true)))

(event Custom|Update%20Citizen%20Costs)

(event EventBeginPlay
  (|CallParentFunction)
  (Variables|Default|SetMeshes (Utilities|Array|MakeArray (Variables|Default|GetBuilding%20Mesh) (Variables|Default|GetStaticMesh) (Variables|Default|GetBlade))))

(event EventAddFarmlandtoWindmill
  (params (Farmland :type Actor%20Object%20Reference))
  (Utilities|Array|Add (Variables|Default|GetFarmland%20Attached) Farmland)
  (Class|BPIUI|UpdateDetailsWidget(Message) (Game|GetGameMode) (Variables|Default|GetBuilding%20Data)))

(fn ConstructionScript
  (|CallParentFunction))

(fn GetAttachedActors
  (return (Variables|Default|GetFarmland%20Attached)))

(fn GetPlacedBuildingsArray
  (return 0))

(fn GetCurrentBuildingtoPlace
  (return 0))

(fn GetPlacementRules
  (return "NewEnumerator0" 0))

(fn GetResourceAmount
  (params (Resource%20to%20Find :type E_Resources%20Enum :default "NewEnumerator15"))
  (return 0.0))

(fn GetSelectedBuildingData
  (return ""))