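; BP_BuildingPlacer is a building placement actor that follows the mouse cursor by snapping onto whatever actor lies beneath it.
; Each tick it runs a complex cursor trace from player controller 0, filtered by its ObjectTypes variable.
; On a valid hit it moves to that actor's origin rather than the impact point, without sweeping; otherwise it stays put.
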(event EventBeginPlay
  (|CallParentFunction) ; This node is disabled and will not be called.\nDrag off pins to build functionality.
)

(event Collision|EventActorBeginOverlap
  (params (OtherActor :type Actor%20Object%20Reference))
  (|CallParentFunction OtherActor) ; This node is disabled and will not be called.\nDrag off pins to build functionality.
)

(event EventTick
  (params (DeltaSeconds :type Float%20%28single-precision%29))
  (bind _returnvalue (Game|GetPlayerController 0))
  (bind _object_types (Variables|Default|GetObject%20Types))
  (bind _hitresult (Class|PlayerController|GetHitResultUnderCursorforObjects _returnvalue _object_types true))
  (bind _hitactor (Collision|BreakHitResult _hitresult))
  (|CallParentFunction DeltaSeconds)
  (Utilities|IsValid _hitactor
    (:Is%20Valid
      (Transformation|SetActorLocation (Transformation|GetActorLocation _hitactor) false false))))

(fn ConstructionScript
  (|CallParentFunction))