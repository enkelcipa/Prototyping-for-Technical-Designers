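; City builder game mode that holds the resource stockpile, build, road and demolition modes, placed buildings and acquired upgrades.
; On play it creates the HUD and starts a looping timer that ticks every placed building and refreshes resource, detail, cost and research widgets.
; It relays placement, selection and resource changes between buildings and HUD via messages.
; Stored upgrades are checked against buildings being placed or given new production or consumption.
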(event Custom|Init:%20References
  ;[0.15 0.15 0.15 0.5] Begin Play and Init
  (bind _asbp_city_builder_controller (Utilities|Casting|CastToBP_CityBuilderController (Game|GetPlayerController 0)))
  (Variables|References|SetPlayer%20Controller _asbp_city_builder_controller))

(event Custom|Init:%20HUD
  ;[0.15 0.15 0.15 0.5] Begin Play and Init
  (bind _returnvalue (UserInterface|CreateWidget "/Game/Blueprints/UI/MainHUD/WBP_HUD.WBP_HUD_C" (Variables|References|GetPlayer%20Controller)))
  (Variables|References|SetHUD _returnvalue)
  (UserInterface|Viewport|AddtoViewport _returnvalue 0))

(event Custom|Tick%20All%20Building%20Resources
  (bind _selected_building (Variables|Default|GetSelected%20Building))
  (bind _current_building_to_place (Variables|Default|GetCurrent%20Building%20to%20Place))
  ;[0.15 0.15 0.15 0.5] Tick all resources
  (Utilities|FlowControl|Sequence
    (:then_0
      ;;[0.15 0.15 0.15 0.5] Tick all building resources
      (for _array_element (Variables|Default|GetPlaced%20Buildings)
        (Utilities|IsValid _array_element
          (:Is%20Valid
            (Class|BPIResources|TickResources(Message) _array_element)))))
    (:then_1
      ;;[0.15 0.15 0.15 0.5] Update Ins + Outs Widget
      (CallFunction|UpdateIns+Outs))
    (:then_2
      ;;[0.15 0.15 0.15 0.5] If details widget is visible, update the widget
      (Utilities|IsValid _selected_building
        (:Is%20Valid
          (CallFunction|UpdateDetailsWidget (Variables|/Game/Blueprints/Buildings/BP_BaseBuilding.BP_BaseBuilding_C|GetBuilding%20Data _selected_building)))))
    (:then_3
      ;;[0.15 0.15 0.15 0.5] Update Resource Cost Widget if Visible
      (if (Widget|IsVisible (Variables|/Game/Blueprints/UI/MainHUD/WBP_HUD.WBP_HUD_C|GetRCostBox (Variables|References|GetHUD)))
        (for _array_element_2 (Class|PanelWidget|GetAllChildren (Variables|/Game/Blueprints/UI/MainHUD/WBP_HUD.WBP_HUD_C|GetRCostBox (Variables|References|GetHUD)))
          (bind _resource (Class|BPIGetters|GetAssignedResource(Message) _array_element_2))
          (bind _amount_found (CallFunction|GetResourceAmount _resource))
          (Utilities|IsValid _current_building_to_place
            (:Is%20Valid
              (bind _building_data (Class|BPIGetters|GetBuildingData(Message) _current_building_to_place))
              (Class|BPIUI|UpdateResourceCostWidget(Message) _array_element_2 _resource (.Value (Utilities|Map|Find (Utilities|Struct|BreakS_BuildingData _building_data) _resource)) _amount_found))))))
    (:then_4
      ;;[0.15 0.15 0.15 0.5] If the research tree is visible, check if the player can afford any upgrades
      (if (Widget|IsVisible (Variables|/Game/Blueprints/UI/MainHUD/WBP_HUD.WBP_HUD_C|GetWBP_ResearchMenu (Variables|References|GetHUD)))
        (Default|CheckUpgradeCosts (Variables|/Game/Blueprints/UI/ResearchTree/WBP_ResearchMenu.WBP_ResearchMenu_C|GetWBP_ResearchTree (Variables|/Game/Blueprints/UI/MainHUD/WBP_HUD.WBP_HUD_C|GetWBP_ResearchMenu (Variables|References|GetHUD))))))))

(event Custom|Start%20Ticking%20Resources
  ;[0.15 0.15 0.15 0.5] Tick all resources
  (bind _returnvalue (Utilities|Time|SetTimerbyEvent (EventDispatchers|CreateEvent :!event Custom|Tick%20All%20Building%20Resources) 2e+01 true))
  (Variables|Default|SetResource%20Timer _returnvalue))

(event EventBeginPlay
  ;[0.15 0.15 0.15 0.5] Begin Play and Init
  (CallFunction|Init:References)
  (CallFunction|Init:HUD)
  (bind (_keypin _valuepin) (Utilities|Map|ForEachLoop(Map) (Variables|Default|GetResources))
    (:then
      (Default|UpdateResources (Variables|/Game/Blueprints/UI/MainHUD/WBP_HUD.WBP_HUD_C|GetWBP_ResourceBar (Variables|References|GetHUD)) _keypin _valuepin))
    (:CompletedPin
      (CallFunction|StartTickingResources))))

(event EventSetCastleBonusResources
  (params (Bonus%20Gained? :type Boolean))
  (Variables|Default|SetCastle%20Resources%20Gained? Bonus%20Gained?))

(event EventPlaceBuilding
  (params (Tile :type Actor%20Object%20Reference))
  ;[0.15 0.15 0.15 0.5] Place Building and add to "Placed Buildings" array
  (Class|BPIBuild|PlaceBuilding(Message) (Variables|Default|GetCurrent%20Building%20to%20Place) Tile)
  (Utilities|Array|Add (Variables|Default|GetPlaced%20Buildings) (Variables|Default|GetCurrent%20Building%20to%20Place))
  ;[0.15 0.15 0.15 0.5] Remove the building from this variable
  (Variables|Default|SetCurrent%20Building%20to%20Place 0)
  (CallFunction|UpdateIns+Outs)
  ;[0.15 0.15 0.15 0.5] Disable widgets
  (CallFunction|ToggleResourceCost false (Utilities|Map|MakeMap "NewEnumerator15" 0.0))
  (CallFunction|TogglePlacementReason false))

(event EventUpdateResources
  (params (Resource :type E_Resources%20Enum :default "NewEnumerator15") (Amount :type Float%20%28double-precision%29) (Reduce? :type Boolean))
  (bind _selected_building (Variables|Default|GetSelected%20Building))
  ;[0.15 0.15 0.15 0.5] Update Resources
  (CallFunction|UpdateResource Resource Amount Reduce?)
  (Utilities|IsValid _selected_building
    (:Is%20Valid
      (CallFunction|UpdateDetailsWidget (Variables|/Game/Blueprints/Buildings/BP_BaseBuilding.BP_BaseBuilding_C|GetBuilding%20Data _selected_building)))))

(event EventToggleDetailsPanel
  (params (Visible? :type Boolean) (Building%20Data :type S%20Building%20Data%20Structure))
  ;[0.15 0.15 0.15 0.5] Details Panel
  (Class|BPIUI|ToggleDetailsPanel(Message) (Variables|References|GetHUD) Visible? Building%20Data)
  (CallFunction|UpdateDetailsWidget Building%20Data))

(event EventToggleRoadMode
  (params (Enabled? :type Boolean))
  ;[0.15 0.15 0.15 0.5] Building Placement and Removal
  (Variables|Default|SetRoad%20Mode? Enabled?))

(event EventToggleBuildMode
  (params (Enabled? :type Boolean))
  ;[0.15 0.15 0.15 0.5] Building Placement and Removal
  (bind _output_get (Variables|Default|SetBuild%20Mode? Enabled?))
  (CallFunction|ToggleBuildModeControls _output_get))

(event EventSetCurrentBuildingtoPlace
  (params (Building%20to%20Place :type Actor%20Object%20Reference))
  ;[0.15 0.15 0.15 0.5] Building Placement and Removal
  (bind _output_get (Variables|Default|SetCurrent%20Building%20to%20Place Building%20to%20Place))
  ;;[0.15 0.15 0.15 0.5] Check which upgrade applies to this building and then apply the upgrade
  (CallFunction|CanUpgrade? _output_get))

(event EventRotateBuilding
  (params (CCW? :type Boolean))
  (bind _current_building_to_place (Variables|Default|GetCurrent%20Building%20to%20Place))
  ;[0.15 0.15 0.15 0.5] Building Placement and Removal
  (Utilities|IsValid _current_building_to_place
    (:Is%20Valid
      (Transformation|SetActorRotation _current_building_to_place (Math|Rotator|MakeRotator 0.0 0.0 (+ (.yaw (Transformation|GetActorRotation _current_building_to_place)) (Math|Float|SelectFloat -6e+01 6e+01 CCW?)))))))

(event EventSetSelectedBuilding
  (params (Clicked%20Building :type BP%20Base%20Building%20Object%20Reference))
  ;[0.15 0.15 0.15 0.5] Details Panel
  (Variables|Default|SetSelected%20Building Clicked%20Building))

(event EventUpdateIns+Outs
  (Default|UpdateIns+Outs (Variables|/Game/Blueprints/UI/MainHUD/WBP_HUD.WBP_HUD_C|GetWBP_ResourceIns+Outs (Variables|References|GetHUD))))

(event EventUpdateResourceConsumption
  (params (New%20Consumption :type Map%20of%20E_Resources%20Enums%20to%20Reals :default "NewEnumerator15"))
  (bind _selected_building (Variables|Default|GetSelected%20Building))
  (bind _selected_building_2 (Variables|Default|GetSelected%20Building))
  (bind _building_data (Variables|/Game/Blueprints/Buildings/BP_BaseBuilding.BP_BaseBuilding_C|GetBuilding%20Data _selected_building))
  ;[0.15 0.15 0.15 0.5] Update Resource Production or Consumption on Selected Building
  (Utilities|Map|Clear (Utilities|Struct|BreakS_BuildingData _building_data))
  (Utilities|Struct|SetmembersinS_BuildingData _building_data New%20Consumption)
  (Class|BPIUI|UpdateDetailsWidget(Message) _selected_building_2 (Variables|/Game/Blueprints/Buildings/BP_BaseBuilding.BP_BaseBuilding_C|GetBuilding%20Data _selected_building_2))
  ;;[0.15 0.15 0.15 0.5] Check for upgrades after setting new production or consumption
  (for _array_element (Variables|Default|GetUpgrades)
    (Class|BPIQuery|CanUpgrade?(Message) _array_element (Variables|Default|GetSelected%20Building))))

(event EventUpdateResourceProduction
  (params (Resource :type Map%20of%20E_Resources%20Enums%20to%20Reals :default "NewEnumerator15") (Button :type Widget%20Object%20Reference))
  (bind _selected_building (Variables|Default|GetSelected%20Building))
  (bind _selected_building_2 (Variables|Default|GetSelected%20Building))
  (bind _building_data (Variables|/Game/Blueprints/Buildings/BP_BaseBuilding.BP_BaseBuilding_C|GetBuilding%20Data _selected_building))
  ;[0.15 0.15 0.15 0.5] Update Resource Production or Consumption on Selected Building
  (Utilities|Map|Clear (Utilities|Struct|BreakS_BuildingData _building_data))
  (Utilities|Struct|SetmembersinS_BuildingData _building_data Resource)
  (Class|BPIUI|UpdateDetailsWidget(Message) _selected_building_2 (Variables|/Game/Blueprints/Buildings/BP_BaseBuilding.BP_BaseBuilding_C|GetBuilding%20Data _selected_building_2))
  ;;[0.15 0.15 0.15 0.5] Check for upgrades after setting new production or consumption
  (for _array_element (Variables|Default|GetUpgrades)
    (Class|BPIQuery|CanUpgrade?(Message) _array_element (Variables|Default|GetSelected%20Building))))

(event EventUpdateDetailsWidget
  (params (Building%20Data :type S%20Building%20Data%20Structure))
  ;[0.15 0.15 0.15 0.5] Details Panel
  (Default|UpdatePanel (Variables|/Game/Blueprints/UI/MainHUD/WBP_HUD.WBP_HUD_C|GetWBP_DetailsPanel (Variables|References|GetHUD)) Building%20Data))

(event EventToggleDemoMode
  (params (Enabled? :type Boolean))
  ;[0.15 0.15 0.15 0.5] Building Placement and Removal
  (Variables|Default|SetDemo%20Mode? Enabled?))

(event EventRemoveBuilding
  (params (Building%20to%20Remove :type Actor%20Object%20Reference))
  ;[0.15 0.15 0.15 0.5] Building Placement and Removal
  (Utilities|Array|RemoveItem (Variables|Default|GetPlaced%20Buildings) Building%20to%20Remove)
  (CallFunction|UpdateIns+Outs))

(event EventToggleResourceCost
  (params (Visible :type Boolean) (Resources :type Map%20of%20E_Resources%20Enums%20to%20Reals :default "NewEnumerator15"))
  ;[0.15 0.15 0.15 0.5] Placement Costs and Reason Widgets
  (Class|BPIUI|ToggleResourceCost(Message) (Variables|References|GetHUD) Visible Resources))

(event EventUpdatePlacementReason
  (params (Valid? :type Boolean) (Placement%20Rule :type Array%20of%20E_PlacementRule%20Enums :default "NewEnumerator0") (Placement%20BPs :type Array%20of%20BP%20Base%20Building%20Class%20References) (Text :type Text))
  ;[0.15 0.15 0.15 0.5] Placement Costs and Reason Widgets
  (Default|UpdatePlacementReason (Variables|References|GetHUD) Valid? Placement%20Rule Placement%20BPs))

(event EventTogglePlacementReason
  (params (Visible? :type Boolean))
  ;[0.15 0.15 0.15 0.5] Placement Costs and Reason Widgets
  (Default|TogglePlacementReason (Variables|References|GetHUD) Visible?))

(event EventAddUpgradetoUpgradesList
  (params (Upgrade%20to%20Add :type Actor%20Object%20Reference))
  (Utilities|Array|Add (Variables|Default|GetUpgrades) Upgrade%20to%20Add))

(event EventCanUpgrade?
  (params (Building%20to%20Upgrade :type Actor%20Object%20Reference))
  (for _array_element (Variables|Default|GetUpgrades)
    (Class|BPIQuery|CanUpgrade?(Message) _array_element Building%20to%20Upgrade)))

(event EventTogglePauseMenu
  (params (Visible? :type Boolean))
  (Game|SetGamePaused Visible?)
  (Default|TogglePauseMenu (Variables|References|GetHUD) Visible?))

(fn ConstructionScript)

(fn UpdateResource
  (params (Resource :type E_Resources%20Enum :default "NewEnumerator0") (Amount :type Float%20%28double-precision%29) (Reduce? :type Boolean))
  (Utilities|Map|Add (Variables|Default|GetResources) Resource (+ (.Value (Utilities|Map|Find (Variables|Default|GetResources) Resource)) (Math|Float|SelectFloat (* Amount -1.0) Amount Reduce?)))
  (Default|UpdateResources (Variables|References|GetHUD) Resource (.Value (Utilities|Map|Find (Variables|Default|GetResources) Resource))))

(fn AdjacenttoRoad?
  (return false))

(fn CanPlayerAfford?
  (bind _current_building_to_place (Variables|Default|GetCurrent%20Building%20to%20Place))
  (Utilities|IsValid _current_building_to_place
    (:Is%20Valid
      (bind _can_afford_ (Class|BPIQuery|CanPlayerAfford?(Message) _current_building_to_place))
      (return _can_afford_))))

(fn GainedBonusResources?
  (return (Variables|Default|GetCastle%20Resources%20Gained?)))

(fn GetAssignedResource
  (return "NewEnumerator15"))

(fn GetBuildingData
  (return ""))

(fn GetController
  (return false))

(fn GetCurrentBuildingtoPlace
  (bind _current_building_to_place (Variables|Default|GetCurrent%20Building%20to%20Place))
  (Utilities|IsValid _current_building_to_place
    (:Is%20Valid
      (return _current_building_to_place))))

(fn GetPlacedBuildingsArray
  (return (Variables|Default|GetPlaced%20Buildings)))

(fn GetPlacementRules
  (return "NewEnumerator0" 0))

(fn GetResourceAmount
  (params (Resource%20to%20Find :type E_Resources%20Enum :default "NewEnumerator15"))
  (return (.Value (Utilities|Map|Find (Variables|Default|GetResources) Resource%20to%20Find))))

(fn GetSelectedBuildingData
  (return (Variables|/Game/Blueprints/Buildings/BP_BaseBuilding.BP_BaseBuilding_C|GetBuilding%20Data (Variables|Default|GetSelected%20Building))))

(fn InBuildMode?
  (return (Variables|Default|GetBuild%20Mode?)))

(fn InDemoMode?
  (return (Variables|Default|GetDemo%20Mode?)))

(fn InRoadMode?
  (return (Variables|Default|GetRoad%20Mode?)))

(fn IsAdjacenttoRuleBP?
  (params (Rule%20BPs :type Array%20of%20Actor%20Class%20References))
  (return false))

(fn TileOccupied?
  (return false))