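; City builder game mode that owns the resource totals, build/road/demolish mode flags, placed buildings and current selection.
; On BeginPlay it creates the HUD, fills the resource bar and starts a looping resource timer; building ticks are delegated to each placed building.
; It handles placement, 60-degree rotation and production edits, pushing resource and building data to the HUD.
; Several query functions, such as adjacency and tile occupancy, are empty or constant stubs.
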(event Custom|Init:%20References
  (bind _asbp_city_builder_controller (Utilities|Casting|CastToBP_CityBuilderController (Game|GetPlayerController 0)))
  (Variables|References|SetPlayer%20Controller _asbp_city_builder_controller))

(event Custom|Init:%20HUD
  (bind _returnvalue (UserInterface|CreateWidget "/Game/Blueprints/UI/WBP_HUD.WBP_HUD_C" (Variables|References|GetPlayer%20Controller)))
  (Variables|References|SetHUD _returnvalue)
  (UserInterface|Viewport|AddtoViewport _returnvalue 0))

(event Custom|Tick%20All%20Building%20Resources
  (bind _selected_building (Variables|Default|GetSelected%20Building))
  (for _array_element (Variables|Default|GetPlaced%20Buildings)
    (Utilities|IsValid _array_element
      (:Is%20Valid
        (Class|BPIResources|TickResources(Message) _array_element))))
  (Utilities|IsValid _selected_building
    (:Is%20Valid
      (CallFunction|UpdateDetailsWidget (Variables|/Game/Blueprints/Buildings/BP_BaseBuilding.BP_BaseBuilding_C|GetBuilding%20Data _selected_building)))))

(event Custom|Start%20Ticking%20Resources
  (bind _returnvalue (Utilities|Time|SetTimerbyEvent (EventDispatchers|CreateEvent :!event Custom|Tick%20All%20Building%20Resources) 5.0 true))
  (Variables|Default|SetResource%20Timer _returnvalue))

(event EventBeginPlay
  (CallFunction|Init:References)
  (CallFunction|Init:HUD)
  (bind (_keypin _valuepin) (Utilities|Map|ForEachLoop(Map) (Variables|Default|GetResources))
    (:then
      (Default|UpdateResources (Variables|/Game/Blueprints/UI/WBP_HUD.WBP_HUD_C|GetWBP_ResourceBar (Variables|References|GetHUD)) _keypin _valuepin))
    (:CompletedPin
      (CallFunction|StartTickingResources))))

(event EventSetCastleBonusResources
  (params (Bonus%20Gained? :type Boolean))
  (Variables|Default|SetCastle%20Resources%20Gained? Bonus%20Gained?))

(event EventPlaceBuilding
  (params (Tile :type Actor%20Object%20Reference))
  (Class|BPIBuild|PlaceBuilding(Message) (Variables|Default|GetCurrent%20Building%20to%20Place) Tile)
  (Utilities|Array|Add (Variables|Default|GetPlaced%20Buildings) (Variables|Default|GetCurrent%20Building%20to%20Place))
  (Variables|Default|SetCurrent%20Building%20to%20Place 0))

(event EventUpdateResources
  (params (Resource :type E_Resources%20Enum :default "NewEnumerator15") (Amount :type Float%20%28double-precision%29) (Reduce? :type Boolean))
  (CallFunction|UpdateResource Resource Amount Reduce?))

(event EventToggleDetailsPanel
  (params (Visible? :type Boolean) (Building%20Data :type S%20Building%20Data%20Structure))
  (Class|BPIUI|ToggleDetailsPanel(Message) (Variables|References|GetHUD) Visible? Building%20Data)
  (CallFunction|UpdateDetailsWidget Building%20Data))

(event EventToggleRoadMode
  (params (Enabled? :type Boolean))
  (Variables|Default|SetRoad%20Mode? Enabled?))

(event EventToggleBuildMode
  (params (Enabled? :type Boolean))
  (bind _output_get (Variables|Default|SetBuild%20Mode? Enabled?))
  (CallFunction|ToggleBuildModeControls _output_get))

(event EventSetCurrentBuildingtoPlace
  (params (Building%20to%20Place :type Actor%20Object%20Reference))
  (Variables|Default|SetCurrent%20Building%20to%20Place Building%20to%20Place))

(event EventRotateBuilding
  (params (CCW? :type Boolean))
  (bind _current_building_to_place (Variables|Default|GetCurrent%20Building%20to%20Place))
  (Utilities|IsValid _current_building_to_place
    (:Is%20Valid
      (Transformation|SetActorRotation _current_building_to_place (Math|Rotator|MakeRotator 0.0 0.0 (+ (.yaw (Transformation|GetActorRotation _current_building_to_place)) (Math|Float|SelectFloat -6e+01 6e+01 CCW?)))))))

(event EventSetSelectedBuilding
  (params (Clicked%20Building :type BP%20Base%20Building%20Object%20Reference))
  (Variables|Default|SetSelected%20Building Clicked%20Building))

(event EventUpdateResourceConsumption
  (params (New%20Consumption :type Map%20of%20E_Resources%20Enums%20to%20Reals :default "NewEnumerator15"))
  (bind _selected_building (Variables|Default|GetSelected%20Building))
  (bind _selected_building_2 (Variables|Default|GetSelected%20Building))
  (bind _building_data (Variables|/Game/Blueprints/Buildings/BP_BaseBuilding.BP_BaseBuilding_C|GetBuilding%20Data _selected_building))
  (Utilities|Map|Clear (Utilities|Struct|BreakS_BuildingData _building_data))
  (Utilities|Struct|SetmembersinS_BuildingData _building_data New%20Consumption)
  (Class|BPIUI|UpdateDetailsWidget(Message) _selected_building_2 (Variables|/Game/Blueprints/Buildings/BP_BaseBuilding.BP_BaseBuilding_C|GetBuilding%20Data _selected_building_2)))

(event EventUpdateResourceProduction
  (params (Resource :type Map%20of%20E_Resources%20Enums%20to%20Reals :default "NewEnumerator15") (Button :type Widget%20Object%20Reference))
  (bind _selected_building (Variables|Default|GetSelected%20Building))
  (bind _selected_building_2 (Variables|Default|GetSelected%20Building))
  (bind _building_data (Variables|/Game/Blueprints/Buildings/BP_BaseBuilding.BP_BaseBuilding_C|GetBuilding%20Data _selected_building))
  (Utilities|Map|Clear (Utilities|Struct|BreakS_BuildingData _building_data))
  (Utilities|Struct|SetmembersinS_BuildingData _building_data Resource)
  (Class|BPIUI|UpdateDetailsWidget(Message) _selected_building_2 (Variables|/Game/Blueprints/Buildings/BP_BaseBuilding.BP_BaseBuilding_C|GetBuilding%20Data _selected_building_2)))

(event EventUpdateDetailsWidget
  (params (Building%20Data :type S%20Building%20Data%20Structure))
  (Default|UpdatePanel (Variables|/Game/Blueprints/UI/WBP_HUD.WBP_HUD_C|GetWBP_DetailsPanel (Variables|References|GetHUD)) Building%20Data))

(event EventToggleDemoMode?
  (params (Enabled? :type Boolean))
  (Variables|Default|SetDemo%20Mode? Enabled?))

(event EventRemoveBuilding
  (params (Building%20to%20Remove :type Actor%20Object%20Reference))
  (Utilities|Array|RemoveItem (Variables|Default|GetPlaced%20Buildings) Building%20to%20Remove))

(fn ConstructionScript)

(fn UpdateResource
  (params (Resource :type E_Resources%20Enum :default "NewEnumerator0") (Amount :type Float%20%28double-precision%29) (Reduce? :type Boolean))
  (Utilities|Map|Add (Variables|Default|GetResources) Resource (+ (.Value (Utilities|Map|Find (Variables|Default|GetResources) Resource)) (Math|Float|SelectFloat (* Amount -1.0) Amount Reduce?)))
  (Default|UpdateResources (Variables|References|GetHUD) Resource (.Value (Utilities|Map|Find (Variables|Default|GetResources) Resource))))

(fn AdjacenttoRoad?
  (return false))

(fn CanPlayerAfford?
  (bind _current_building_to_place (Variables|Default|GetCurrent%20Building%20to%20Place))
  (Utilities|IsValid _current_building_to_place
    (:Is%20Valid
      (bind _can_afford_ (Class|BPIQuery|CanPlayerAfford?(Message) _current_building_to_place))
      (return _can_afford_))))

(fn GainedBonusResources?
  (return (Variables|Default|GetCastle%20Resources%20Gained?)))

(fn GetAttachedActors
  (return 0))

(fn GetCurrentBuildingtoPlace
  (bind _current_building_to_place (Variables|Default|GetCurrent%20Building%20to%20Place))
  (Utilities|IsValid _current_building_to_place
    (:Is%20Valid
      (return _current_building_to_place))))

(fn GetPlacedBuildingsArray
  (return (Variables|Default|GetPlaced%20Buildings)))

(fn GetPlacementRules
  (return "NewEnumerator0" 0))

(fn GetResourceAmount
  (params (Resource%20to%20Find :type E_Resources%20Enum :default "NewEnumerator15"))
  (return (.Value (Utilities|Map|Find (Variables|Default|GetResources) Resource%20to%20Find))))

(fn GetSelectedBuildingData
  (return (Variables|/Game/Blueprints/Buildings/BP_BaseBuilding.BP_BaseBuilding_C|GetBuilding%20Data (Variables|Default|GetSelected%20Building))))

(fn InBuildMode?
  (return (Variables|Default|GetBuild%20Mode?)))

(fn InDemoMode?
  (return (Variables|Default|GetDemo%20Mode?)))

(fn InRoadMode?
  (return (Variables|Default|GetRoad%20Mode?)))

(fn IsAdjacenttoRuleBP?
  (params (Rule%20BPs :type Array%20of%20Actor%20Class%20References))
  (return false))

(fn TileOccupied?
  (return false))